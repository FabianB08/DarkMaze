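; Waypoint component meant to draw a navigation path from its owning actor to a goal location.
; GetPath runs a synchronous navmesh path query, and Server_GetPath forwards to it.
; OwnerCreateWaypoints turns path points into a height-offset, constant-type spline and adds spline mesh components on a waypoint manager actor.
; CreateWaypoint is empty: the manager-spawning setup and the hand-off from path result to spline building are disconnected and never run.
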(event `Server_GetPath`
  (params (TargetLocation :type "Vector Structure"))
  (`self.GetPath` TargetLocation))

(event `CreateWaypoint`
  (params (GoalLocation :type "Vector Structure") (goalDistance :type "Float (double-precision)") (UpdateDistance :type "Float (double-precision)") (UpdateInterval :type "Float (double-precision)") (Z_offset :type "Float (double-precision)")))

(event `GetPath`
  (params (TargetLocation :type "Vector Structure"))
  (bind _returnvalue (`NavigationSystemV1.FindPathToLocationSynchronously` (`Actor.K2_GetActorLocation` (`self.GetOwner`)) TargetLocation null null)))

(event `OwnerCreateWaypoints`
  (params (Path :type "Array of Vector Structure"))
  (bind _splinecomp (`self.SplineComp`))
  (bind _output_get (set `self.Path` Path))
  (set `self.WaypointStartLocation` (`|GetArrayItem` _output_get))
  (`/Game/MazeGenerator/Blueprints/Waypoints/Blueprints/BP_waypoint_Manager.RemoveWaypoint` (`self.Bp_WaypointManager`))
  (for (_array_element _array_index) (`self.Path`)
    (`SplineComponent.AddSplinePointAtIndex` _splinecomp (+ _array_element (`KismetMathLibrary.MakeVector` 0.0 0.0 (`self.Z_offset`))) _array_index "World" false)
    (`SplineComponent.SetSplinePointType` _splinecomp _array_index "Constant" false))
  (`SplineComponent.UpdateSpline` (`self.SplineComp`))
  (for _ (range (`KismetArrayLibrary.Array_LastIndex` (`self.Path`)))
    (`|AddComponentByClass` :`self` (`self.Bp_WaypointManager`) :`Class` "/Script/Engine.SplineMeshComponent" :`bManualAttachment` true)
    (`KismetArrayLibrary.Array_Add` (`/Game/MazeGenerator/Blueprints/Waypoints/Blueprints/BP_waypoint_Manager.SplineMeshes` (`self.Bp_WaypointManager`)))))